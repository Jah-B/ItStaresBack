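; Base game mode that starts dungeon generation on BeginPlay and handles game setup, defeat and an item respawner registry.
; SetupGame caches the player and enemy, then spawns a collisionless lantern attached unheld to the player and added to their inventory after short delays.
; It also has the Planner and WorldState actors set their references and starts the enemy behavior tree.
; Defeat loads ThirdPersonMap as a level instance.
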(event EventBeginPlay
  (bind _returnvalue (Actor|GetActorOfClass "/Game/ProcGen/Dungeon_Generator.Dungeon_Generator_C"))
  (Default|BeginDungeonGeneration _returnvalue))

(event EventSetupGame
  (Utilities|FlowControl|Sequence
    (:then_0
      (bind _asbp_player (Utilities|Casting|CastToBP_Player (Game|GetPlayerCharacter 0)))
      (Variables|Default|SetPlayer%20Reference _asbp_player)
      (bind _returnvalue (Actor|GetActorOfClass "/Game/Enemy/BP_Enemy.BP_Enemy_C"))
      (Variables|Default|SetEnemy%20Reference _returnvalue))
    (:then_1
      (Utilities|FlowControl|Delay 0.1)
      (bind _returnvalue_2 (Game|SpawnActorfromClass "/Game/Items/BPs/BP_Lantern.BP_Lantern_C" (Math|Transform|MakeTransform "0, 0, 0" "0, 0, 0" "1.000000,1.000000,1.000000") "Undefined" "MultiplyWithRoot" 0 "NewEnumerator3" 0))
      (Utilities|FlowControl|Delay 0.1)
      (Collision|SetCollisionEnabled (Variables|/Game/Items/BPs/BP_ItemActor.BP_ItemActor_C|GetStaticMesh _returnvalue_2) "NoCollision")
      (Default|AttachLanternUnheld (Variables|Default|GetPlayer%20Reference) _returnvalue_2)
      (Class|BPIInventory|AddItem(Message) (Actor|GetComponentbyClass (Variables|Default|GetPlayer%20Reference) "/Game/Components/BPC_Inventory.BPC_Inventory_C") _returnvalue_2))
    (:then_2
      (bind _returnvalue_3 (Actor|GetActorOfClass "/Game/GOAP/BP_Planner.BP_Planner_C"))
      (Default|SetReferencesonBeginGame _returnvalue_3)
      (bind _returnvalue_4 (Actor|GetActorOfClass "/Game/GOAP/BP_WorldState.BP_WorldState_C"))
      (Default|SetReferencesonBeginGame _returnvalue_4)
      (bind _asbp_enemy_controller (Utilities|Casting|CastToBP_EnemyController (AI|GetAIController (Variables|Default|GetEnemy%20Reference)))
        (:then
          (Default|RunEnemyBehaviorTree _asbp_enemy_controller))
        (:CastFailed
          (Development|PrintString "Failed"))))))

(event EventEndGame
  (params (Ending :type Enum_Endings%20Enum :default "NewEnumerator0"))
  (switch Utilities|FlowControl|Switch|SwitchonEnum_Endings Ending
    (:NewEnumerator1
      (Class|LevelStreamingDynamic|LoadLevelInstancebySoftObjectPtr "/Game/ThirdPerson/Maps/ThirdPersonMap.ThirdPersonMap" "0, 0, 0" "0, 0, 0" "" 0 false))))

(event EventAddItemRespawner
  (params (Respawner :type BP%20Respawner%20Object%20Reference))
  (Utilities|Array|Add (Variables|Default|GetRespawners) Respawner))

(fn ConstructionScript)

(fn GetAllItemRespawners
  (return (Variables|Default|GetRespawners)))