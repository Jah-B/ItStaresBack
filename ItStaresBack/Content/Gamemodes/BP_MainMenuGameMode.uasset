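; Main menu game mode that puts the WBP_Menu widget on screen and shows the mouse cursor for player 0.
; The widget is created, stored in MenuReference and added to the viewport in the Construction Script, while BeginPlay only enables the cursor.
; MessageFadeAnimation forwards to the menu's FadeAnimation with a false argument.
; GetAllItemRespawners and GetEnemy are empty stubs, and Tick does nothing.
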(event EventBeginPlay
  (Variables|/Script/Engine.PlayerController|SetbShowMouseCursor (Game|GetPlayerController 0) true))

(event EventTick
  (params (DeltaSeconds :type Float%20%28single-precision%29)))

(event EventMessageFadeAnimation
  (params (Fade%20In/Out :type Boolean))
  (Default|FadeAnimation (Variables|Default|GetMenu%20Reference) false))

(fn ConstructionScript
  (bind _returnvalue (Game|ConstructObjectfromClass "/Game/UI/Menu/WBP_Menu.WBP_Menu_C"))
  (Variables|Default|SetMenu%20Reference _returnvalue)
  (UserInterface|Viewport|AddtoViewport _returnvalue 0))

(fn GetAllItemRespawners
  (return 0))

(fn GetEnemy
  (return 0))