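; Held-item component whose useItem event applies the effect of the player's equipped item, ignoring the Lantern.
; Other items are detached and moved to world origin rather than destroyed, then branched on EnumName.
; Bear Trap spawns BP_BearTrap at the player character's trace hit, falling back to the player's location.
; Flint and Steel checks BPC_Inventory for a lantern and lights the BP_Lantern found in the world, otherwise printing an effect placeholder.
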(event Custom|useItem
  (params (EquippedItem :type BP%20Item%20Actor%20Object%20Reference))
  (bind _returnvalue (Game|GetPlayerCharacter 0))
  (if (not (Utilities|Enum|Equal(Enum) (Variables|/Game/Items/BPs/BP_ItemActor.BP_ItemActor_C|GetEnumName EquippedItem) "NewEnumerator3"))
    (Transformation|DetachFromActor EquippedItem "KeepRelative" "KeepRelative" "KeepRelative")
    (Transformation|SetActorLocation EquippedItem "0, 0, 0" false false)
    (switch Utilities|FlowControl|Switch|SwitchonEnum_Items (Variables|/Game/Items/BPs/BP_ItemActor.BP_ItemActor_C|GetEnumName EquippedItem)
      (:NewEnumerator1
        (bind (_spawn_location _hit_) (Class|BPIItemInteraction|SpawnBearTrap(Message) _returnvalue))
        (if _hit_
          (Game|SpawnActorfromClass "/Game/Items/BPs/BP_BearTrap.BP_BearTrap_C" (Math|Transform|MakeTransform _spawn_location "0, 0, 0" "1.000000,1.000000,1.000000") "Undefined" "MultiplyWithRoot" 0 0)
          (else
            (Game|SpawnActorfromClass "/Game/Items/BPs/BP_BearTrap.BP_BearTrap_C" (Math|Transform|MakeTransform (Transformation|GetActorLocation _returnvalue) "0, 0, 0" "1.000000,1.000000,1.000000") "Undefined" "MultiplyWithRoot" 0 0))))
      (:NewEnumerator2
        (bind _have_lantern_ (Default|CheckforLantern (Actor|GetComponentbyClass (Game|GetPlayerCharacter 0) "/Game/Components/BPC_Inventory.BPC_Inventory_C")))
        (if _have_lantern_
          (bind _returnvalue_2 (Actor|GetActorOfClass "/Game/Items/BPs/BP_Lantern.BP_Lantern_C"))
          (Default|LightLanternFlame _returnvalue_2)
          (Development|PrintString "it didnt work oh i see")
          (Transformation|DetachFromActor EquippedItem "KeepRelative" "KeepRelative" "KeepRelative")
          (Transformation|SetActorLocation EquippedItem "0, 0, 0" false false)
          (else
            ;[1 1 1] PLAY A SPECIAL EFFECT
            (Development|PrintString "PLAY A SPECIAL EFFECT")
            (Transformation|DetachFromActor EquippedItem "KeepRelative" "KeepRelative" "KeepRelative")
            (Transformation|SetActorLocation EquippedItem "0, 0, 0" false false)))))))

(event EventTick
  (params (DeltaSeconds :type Float%20%28single-precision%29)))