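; BPC_Inventory is an inventory component that stores held items and drives the W_InventoryMenu widget created at BeginPlay.
; AddItem records an item and fills a widget slot, while MoveItemBackToInventory only refills a slot.
; OpenInventory toggles the menu, input mode and mouse cursor.
; Helpers remove items, add the spawned lantern and check for one by enum; the logic attaching it to BP_Player is disconnected.
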(event Custom|OpenInventory
  (bind _returnvalue (Game|GetPlayerController 0))
  (if (Variables|Default|GetInvOpen?)
    (Variables|Default|SetInvOpen? false)
    (Widget|RemovefromParent (Variables|Default|GetInventoryWidget))
    (Input|SetInputModeGameOnly (Game|GetPlayerController 0) false)
    (Variables|/Script/Engine.PlayerController|SetbShowMouseCursor (Game|GetPlayerController 0) false)
    (else
      (Variables|Default|SetInvOpen? true)
      (UserInterface|Viewport|AddtoViewport (Variables|Default|GetInventoryWidget) 0)
      (Input|SetInputModeGameandUI _returnvalue 0 "DoNotLock" true false)
      (Variables|/Script/Engine.PlayerController|SetbShowMouseCursor _returnvalue true))))

(event EventBeginPlay
  (bind _returnvalue (UserInterface|CreateWidget "/Game/UI/Inventory/W_InventoryMenu.W_InventoryMenu_C"))
  (Variables|Default|SetInventoryWidget _returnvalue))

(event EventTick
  (params (DeltaSeconds :type Float%20%28single-precision%29)))

(event EventAddItem
  (params (Item :type BP%20Item%20Actor%20Object%20Reference))
  (Utilities|Array|Add (Variables|Default|GetHeldItems) Item)
  (Default|AddIteminSlot (Variables|Default|GetInventoryWidget) Item))

(fn MoveItemBacktoInventory
  (params (Item%20Actor :type BP%20Item%20Actor%20Object%20Reference))
  (Default|AddIteminSlot (Variables|Default|GetInventoryWidget) Item%20Actor))

(fn AddLanterntoPlayer
  (params (Spawned%20Lantern :type BP%20Item%20Actor%20Object%20Reference))
  ;[1 1 1] Initial Lantern Spawn
  (CallFunction|AddItem Spawned%20Lantern))

(fn CheckforLantern
  (bind _array_element (Utilities|Array|ForEachLoopwithBreak (Variables|Default|GetHeldItems) :!label _label)
    (:LoopBody
      (if (Utilities|Enum|Equal(Enum) (Variables|/Game/Items/BPs/BP_ItemActor.BP_ItemActor_C|GetEnumName _array_element) "NewEnumerator3")
        (LocalVariables|SetLantern%20in%20Inventory true)
        (goto _label Break)))
    (:Completed
      (return (LocalVariables|GetLantern%20in%20Inventory)))))

(fn RemovefromInventoryIndex
  (params (ItemActor :type BP%20Item%20Actor%20Object%20Reference))
  (bind _output_get (LocalVariables|SetStoredItem 0))
  (Utilities|Array|RemoveItem (Variables|Default|GetHeldItems) ItemActor)
  (return _output_get))