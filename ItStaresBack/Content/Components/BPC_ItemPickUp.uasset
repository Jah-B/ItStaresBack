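; Item pick-up component that lets its owner select, collect and drop items implementing BPI_Items.
; Each Tick, a short box trace from the eye viewpoint updates the selected item through interface messages.
; Interact adds it to BPC_Inventory, shows its name in W_InventoryItems and moves the actor to world origin instead of destroying it.
; Drop calls RemoveItem without an item; disconnected multi-trace, nearest-item logic never runs.
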(event Custom|Remove%20Item
  (params (Item%20Actor :type BP%20Item%20Actor%20Object%20Reference))
  (bind _returnvalue (Components|GetOwner))
  ;[1 1 1] Drop Item
  (Default|RemovefromInventoryIndex (Actor|GetComponentbyClass _returnvalue "/Game/Components/BPC_Inventory.BPC_Inventory_C") Item%20Actor)
  (Transformation|SetActorLocation Item%20Actor (+ (Transformation|GetActorLocation _returnvalue) (* (Transformation|GetActorForwardVector _returnvalue) 2.0)) false false))

(event Input|EnhancedActionEvents|EnhancedInputActionIA_Interact
  (params (ActionValue :type Boolean) (ElapsedSeconds :type Float%20%28double-precision%29) (TriggeredSeconds :type Float%20%28double-precision%29) (InputAction :type Input%20Action%20Object%20Reference :default "/Game/Player/Input/Actions/IA_Interact.IA_Interact"))
  (bind _ui_pop_up (Variables|Default|GetUI%20Pop%20Up))
  ;[1 1 1] If player looking at an item, add it to inventory. Then set selected item to be null
  (Utilities|IsValid (Variables|Default|GetSelectedItem)
    (:Is%20Valid
      (bind _selecteditem (Class|BPIItems|PickUpItem(Message) (Variables|Default|GetSelectedItem)))
      (Default|AddItem (Actor|GetComponentbyClass (Components|GetOwner) "/Game/Components/BPC_Inventory.BPC_Inventory_C") _selecteditem)
      (bind _name (Class|BPIItems|OutInfo(Message) (Variables|Default|GetSelectedItem)))
      (Class|BPIUI|GetName(Message) _ui_pop_up _name)
      (UserInterface|Viewport|AddtoViewport _ui_pop_up 0)
      (Class|BPIItems|StopBobbing(Message) (Variables|Default|GetSelectedItem))
      (Transformation|SetActorLocation (Variables|Default|GetSelectedItem) "0, 0, 0" false false)
      (Class|BPIItems|DeselectItem(Message) (Variables|Default|GetSelectedItem))
      (Variables|Default|SetSelectedItem 0))))

(event Input|EnhancedActionEvents|EnhancedInputActionIA_DropItem
  (params (ActionValue :type Boolean) (ElapsedSeconds :type Float%20%28double-precision%29) (TriggeredSeconds :type Float%20%28double-precision%29) (InputAction :type Input%20Action%20Object%20Reference :default "/Game/Player/Input/Actions/IA_DropItem.IA_DropItem"))
  ;[1 1 1] Drop Item
  (CallFunction|RemoveItem))

(event EventBeginPlay
  (bind _returnvalue (UserInterface|CreateWidget "/Game/UI/Inventory/W_InventoryItems.W_InventoryItems_C" (Game|GetPlayerController 0)))
  (Variables|Default|SetUI%20Pop%20Up _returnvalue))

(event EventTick
  (params (DeltaSeconds :type Float%20%28single-precision%29))
  (bind _returnvalue (Components|GetOwner))
  (bind (_outlocation _outrotation) (Actor|GetActorEyesViewPoint _returnvalue))
  ;[1 1 1] Box Trace from player's eyes
  (bind (_outhit _returnvalue_2) (Class|KismetSystemLibrary|BoxTraceSingleforObjects _outlocation (+ _outlocation (* (Math|Vector|GetForwardVector _outrotation) 1.5e+02)) "10.000000,10.000000,30.000000" _outrotation (Utilities|Array|MakeArray "ObjectTypeQuery2") false 0 "None" true))
  ;[1 1 1] Check if there was a hit, and check if it was an item
  (if _returnvalue_2
    (if (Utilities|DoesObjectImplementInterface (.HitActor (Collision|BreakHitResult _outhit)) "/Game/Interfaces/BPI_Items.BPI_Items_C")
      (if (Utilities|DoesObjectImplementInterface (Variables|Default|GetSelectedItem) "/Game/Interfaces/BPI_Items.BPI_Items_C")
        (Class|BPIItems|DeselectItem(Message) (Variables|Default|GetSelectedItem)))
      (bind _output_get (Variables|Default|SetSelectedItem (.HitActor (Collision|BreakHitResult _outhit))))
      (Class|BPIItems|SelectItem(Message) _output_get))
    (else
      ;[1 1 1] When player is looking at NOTHING, deselect selected item
      (Class|BPIItems|DeselectItem(Message) (Variables|Default|GetSelectedItem))
      (Variables|Default|SetSelectedItem 0))))