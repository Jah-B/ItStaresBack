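; BP_ItemActor is an item actor that takes on a random identity from the DT_Items data table at BeginPlay.
; The chosen row supplies its name, durability and static mesh.
; SelectItem and DeselectItem swap highlight overlay materials on the mesh.
; OutInfo returns the name and durability, and PickUpItem returns the actor itself without removing or altering it.
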(event EventBeginPlay
  (bind _outrownames (DataTable|GetDataTableRowNames "/Game/Items/DT_Items.DT_Items"))
  (bind _returnvalue (Utilities|GetDataTableRow "/Game/Items/DT_Items.DT_Items" (.OutItem (Utilities|Array|Random _outrownames)))
    (:then
      (Variables|Default|SetItemName (.Name (Utilities|Struct|BreakStruct_Items _returnvalue)))
      (Variables|Default|SetDurability (.Durability (Utilities|Struct|BreakStruct_Items _returnvalue)))
      (Components|StaticMesh|SetStaticMesh (Variables|Default|GetStaticMesh) (.StaticMesh (Utilities|Struct|BreakStruct_Items _returnvalue))))))

(event Collision|EventActorBeginOverlap
  (params (OtherActor :type Actor%20Object%20Reference)))

(event EventTick
  (params (DeltaSeconds :type Float%20%28single-precision%29)))

(event EventSelectItem
  (Rendering|Material|SetOverlayMaterial (Variables|Default|GetStaticMesh) "/Game/Items/M_HighlightSelected.M_HighlightSelected" :!class /Script/Engine.MeshComponent))

(event EventDeselectItem
  (Rendering|Material|SetOverlayMaterial (Variables|Default|GetStaticMesh) "/Game/Items/M_HighlightUnselected.M_HighlightUnselected" :!class /Script/Engine.MeshComponent))

(fn ConstructionScript)

(fn OutInfo
  (return (Variables|Default|GetItemName) (Variables|Default|GetDurability)))

(fn PickUpItem
  (return self))