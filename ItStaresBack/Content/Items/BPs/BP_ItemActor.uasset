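; World item actor that randomizes itself from the DT_Items data table and can be highlighted and picked up.
; On BeginPlay, unless its enum equals one specific value, it copies name, durability, static mesh and enum from a random row.
; Select and deselect events swap the mesh's overlay highlight material, while functions return its info or the actor itself for pickup.
; The same randomization sits unconnected in the construction script.
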(event EventBeginPlay
  (if (not (Utilities|Enum|Equal(Enum) (Variables|Default|GetEnumName) "NewEnumerator3"))
    (bind _outrownames (DataTable|GetDataTableRowNames "/Game/Items/Structs-DataTables/DT_Items.DT_Items"))
    (bind _returnvalue (Utilities|GetDataTableRow "/Game/Items/Structs-DataTables/DT_Items.DT_Items" (.OutItem (Utilities|Array|Random _outrownames)))
      (:then
        (Variables|Default|SetItemName (.Name (Utilities|Struct|BreakStruct_Items _returnvalue)))
        (Variables|Default|SetDurability (.Durability (Utilities|Struct|BreakStruct_Items _returnvalue)))
        (Components|StaticMesh|SetStaticMesh (Variables|Default|GetStaticMesh) (.StaticMesh (Utilities|Struct|BreakStruct_Items _returnvalue)))
        (Variables|Default|SetEnumName (.EnumName (Utilities|Struct|BreakStruct_Items _returnvalue)))))))

(event EventSelectItem
  (Rendering|Material|SetOverlayMaterial (Variables|Default|GetStaticMesh) "/Game/Items/Materials/M_HighlightSelected.M_HighlightSelected" :!class /Script/Engine.MeshComponent))

(event EventDeselectItem
  (Rendering|Material|SetOverlayMaterial (Variables|Default|GetStaticMesh) "/Game/Items/Materials/M_HighlightUnselected.M_HighlightUnselected" :!class /Script/Engine.MeshComponent))

(fn ConstructionScript)

(fn OutInfo
  (return (Variables|Default|GetItemName) (Variables|Default|GetDurability)))

(fn PickUpItem
  (return self))