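; Bear trap item actor that arms itself two seconds after BeginPlay and springs when an actor overlaps its trigger.
; The first overlap disarms it and sends BearTrapTriggerMessage to that actor.
; A true reply plays the closing animation and gory snap sound, then destroys the trap after a delay.
; A false reply leaves the trap in place but disarmed, as nothing re-arms it.
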(event OnComponentBeginOverlap(TrapTrigger)
  (params (OverlappedComponent :type Primitive%20Component%20Object%20Reference) (OtherActor :type Actor%20Object%20Reference) (OtherComp :type Primitive%20Component%20Object%20Reference) (OtherBodyIndex :type Integer) (bFromSweep :type Boolean) (SweepResult :type Hit%20Result%20Structure%20%28by%20ref%29))
  (if (Variables|Default|GetRigged?)
    (Variables|Default|SetRigged? false)
    (bind _valid (Class|BPIItemInteraction|BearTrapTrigger(Message) OtherActor))
    (if _valid
      (Components|Animation|PlayAnimation (Variables|Default|GetSkeletalMesh) "/Game/Assets/Models/Items/Beartrap/Animations/Item_Trap_Anim_Close.Item_Trap_Anim_Close" false)
      (Class|FMODBlueprintStatics|PlayEventatLocation "/Game/FMOD/Events/Beartrap_Close_With_Gore.Beartrap_Close_With_Gore" (Math|Transform|MakeTransform (Transformation|GetActorLocation) "0, 0, 0" "1.000000,1.000000,1.000000"))
      (Utilities|FlowControl|Delay 2.0)
      (Actor|DestroyActor))))

(event EventBeginPlay
  (Utilities|FlowControl|Delay 2.0)
  (Variables|Default|SetRigged? true))

(fn ConstructionScript)