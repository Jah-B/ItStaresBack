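; Planner for the enemy AI that selects the enemy's next action from current player, enemy and world state.
; On a 0.1-second tick it copies perception, trap and roar flags and the investigation list from BP_Player, BP_Enemy and BP_WorldState.
; GeneratePlan is a fixed-priority branch chain rather than a GOAP search: trapped, roaring chase, flee, chase, stalk, investigate, patrol.
; Investigation passes the nearest in-range investigation to the enemy, otherwise falling back to patrol.
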(event Custom|Set%20References%20on%20Begin%20Game
  (Utilities|FlowControl|Sequence
    (:then_0
      (bind _returnvalue (Actor|GetActorOfClass "/Game/Player/BP_Player.BP_Player_C"))
      (bind _output_get (Variables|Ref|SetAs%20BP%20Player _returnvalue))
      (Development|PrintString (Utilities|GetDisplayName _output_get))
      (bind _returnvalue_2 (Actor|GetActorOfClass "/Game/Enemy/BP_Enemy.BP_Enemy_C"))
      (Variables|Ref|SetAs%20BP%20Enemy _returnvalue_2)
      (Actor|Tick|SetActorTickEnabled true)
      (bind _returnvalue_3 (Actor|GetActorOfClass "/Game/GOAP/BP_WorldState.BP_WorldState_C"))
      (Variables|Ref|SetAs%20World%20State _returnvalue_3))
    (:then_1
      (Actor|Tick|SetActorTickInterval 0.1))))

(event EventTick
  (params (DeltaSeconds :type Float%20%28single-precision%29))
  (CallFunction|UpdateVariables))

(fn ConstructionScript)

(fn GeneratePlan
  (params (Agent%20Request :type Actor%20Object%20Reference))
  (bind _investigations (Variables|WorldState|GetInvestigations))
  (bind _as_bp_enemy (Variables|Ref|GetAs%20BP%20Enemy))
  (bind _returnvalue (Transformation|GetActorLocation _as_bp_enemy))
  (bind (_distance _returnvalue_2) (Actor|FindNearestActor _returnvalue _investigations))
  (if (Variables|Enemy|GetEnemyTrapped)
    (return (Utilities|Enum|LiteralenumEnum_Actions "NewEnumerator2") 0)
    (elif (Variables|Enemy|GetRoaring%20Chase)
      ;[1 1 1] Roaring Chase
      (return (Utilities|Enum|LiteralenumEnum_Actions "NewEnumerator6") 0)
      (elif (Variables|Player|GetCan%20See%20Enemy)
        ;[1 1 1] Flee
        (return (Utilities|Enum|LiteralenumEnum_Actions "NewEnumerator4") 0)
        (elif (Variables|Enemy|GetChase%20Player)
          ;[1 1 1] Chase
          (return (Utilities|Enum|LiteralenumEnum_Actions "NewEnumerator3") 0)
          (elif (Variables|Enemy|GetCan%20See%20Player)
            ;[1 1 1] Stalk
            (return (Utilities|Enum|LiteralenumEnum_Actions "NewEnumerator2") 0)
            (elif (Variables|Default|GetInvestigation%20Available)
              ;[1 1 1] Investigation - Find the closest possible investigation and see if its in range
              (if (<= _distance 4e+03)
                (bind _self_actor (Class|BPIGOAP|GetInvestigationActorThroughActor(Message) _returnvalue_2))
                (Class|BPIGOAP|SetSelectedInvestigationActor(Message) (Variables|Ref|GetAs%20BP%20Enemy) _self_actor)
                (return (Utilities|Enum|LiteralenumEnum_Actions "NewEnumerator1") _returnvalue_2)
                (else
                  ;[1 1 1] Patrol
                  (return (Utilities|Enum|LiteralenumEnum_Actions "NewEnumerator0") 0)))
              (else
                ;[1 1 1] Patrol
                (return (Utilities|Enum|LiteralenumEnum_Actions "NewEnumerator0") 0)))))))))

(fn UpdateVariables
  (bind _as_bp_enemy (Variables|Ref|GetAs%20BP%20Enemy))
  (Variables|Enemy|SetCan%20See%20Player (Variables|/Game/Enemy/BP_Enemy.BP_Enemy_C|GetCan%20See%20Player _as_bp_enemy))
  (Variables|Player|SetCan%20See%20Enemy (Variables|/Game/Player/BP_Player.BP_Player_C|GetCan%20See%20Enemy (Variables|Ref|GetAs%20BP%20Player)))
  (Variables|Enemy|SetEnemyTrapped (Variables|/Game/Enemy/BP_Enemy.BP_Enemy_C|GetTrapped _as_bp_enemy))
  (Variables|Enemy|SetRoaring%20Chase (Variables|/Game/Enemy/BP_Enemy.BP_Enemy_C|GetRoaringChase _as_bp_enemy))
  (Variables|Default|SetInvestigation%20Available (not (Utilities|Array|IsEmpty (Variables|/Game/GOAP/BP_WorldState.BP_WorldState_C|GetInvestigations (Variables|Ref|GetAs%20World%20State)))))
  (Variables|WorldState|SetInvestigations (Variables|/Game/GOAP/BP_WorldState.BP_WorldState_C|GetInvestigations (Variables|Ref|GetAs%20World%20State))))

(fn OutputVariables
  (return (Variables|Player|GetCan%20See%20Enemy) (Variables|Enemy|GetCan%20See%20Player) (Variables|WorldState|GetAlerted) (Variables|Enemy|GetEnemyTrapped) false))