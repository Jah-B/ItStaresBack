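; BP_WorldState is a GOAP world-state Blueprint that tracks investigation actors and a reference to the enemy.
; SetReferencesonBeginGame caches every BP_InvestigationParent and one BP_Enemy found in the level.
; UseInvestigationActor removes Shrine-type investigations from that list when used.
; The getters for enemy keys, enemy type, planner and investigation actors are stubs returning default or empty values.
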(event Custom|Set%20References%20on%20Begin%20Game
  (Utilities|FlowControl|Sequence
    (:then_0
      (bind _outactors (Actor|GetAllActorsOfClass "/Game/ProcGen/Investigation/BP_InvestigationParent.BP_InvestigationParent_C"))
      (for _array_element _outactors
        (Utilities|Array|Add (Variables|Default|GetInvestigations) _array_element)))
    (:then_1
      (bind _returnvalue (Actor|GetActorOfClass "/Game/Enemy/BP_Enemy.BP_Enemy_C"))
      (Variables|Default|SetEnemy%20Reference _returnvalue))))

(event Collision|EventActorBeginOverlap
  (params (OtherActor :type Actor%20Object%20Reference)))

(event EventTick
  (params (DeltaSeconds :type Float%20%28single-precision%29)))

(fn ConstructionScript)

(fn UseInvestigationActor
  (params (Investigation%20Actor :type Actor%20Object%20Reference))
  (bind _asbp_investigation_parent (Utilities|Casting|CastToBP_InvestigationParent Investigation%20Actor)
    (:then
      (switch Utilities|FlowControl|Switch|SwitchonEnum_PossibleInvestigations (Variables|/Game/ProcGen/Investigation/BP_InvestigationParent.BP_InvestigationParent_C|GetInvestigation%20Type _asbp_investigation_parent)
        (:NewEnumerator0
          (Utilities|Array|RemoveItem (Variables|Default|GetInvestigations) _asbp_investigation_parent))))
    (:CastFailed
      (Development|PrintString "cast failed"))))

(fn GetEnemyKeys
  (return false))

(fn GetEnemyType
  (return "NewEnumerator0"))

(fn GetInvestigationActorThroughActor
  (return 0))

(fn GetPlanner
  (return 0))

(fn GetSelectedInvestigationActor
  (return 0))