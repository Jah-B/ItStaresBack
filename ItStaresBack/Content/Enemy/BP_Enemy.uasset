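; Enemy character that hunts the player, exposing sight and investigation state and keeping a reference to BP_Planner.
; Sight perception sets CanSeePlayer with a delayed loss check, and the selected action sets movement speed.
; Looping timer traces deliver chase and crawling hits, while other timers end roaring chase and bear-trap holds, which leave it crawling.
; It also records evolutions with player feedback, handles death, and toggles custom-depth X-ray.
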(event OnTargetPerceptionUpdated(SightPerception)
  (params (Actor :type Actor%20Object%20Reference) (Stimulus :type AI%20Stimulus%20Structure))
  (if (.bSuccessfullySensed (Utilities|Struct|BreakAIStimulus Stimulus))
    (Utilities|Casting|CastToBP_Player Actor)
    (Variables|Default|SetCan%20See%20Player true :!label _label)
    (else
      (Utilities|FlowControl|Delay 0.5)
      (if (Utilities|Array|ContainsItem (Class|AIPerceptionComponent|GetPerceivedHostileActors (Variables|Default|GetSight%20Perception)) (Game|GetPlayerCharacter 0))
        (goto _label)
        (else
          (Variables|Default|SetCan%20See%20Player false))))))

(event Custom|Begin%20Trap%20Duration
  ;[1 1 1] Remove Trap when timer runs out
  (bind _returnvalue (Utilities|Time|SetTimerbyEvent (delegate Custom|Remove%20Trap) 1e+01))
  (Variables|Timers|SetTrap%20Removal%20Timer _returnvalue))

(event Custom|Crawl%20Hit%20Trace
  (bind _returnvalue (Transformation|GetActorLocation))
  ;[1 1 1] Hit box for when enemy is crawling
  (bind (_outhit _returnvalue_2) (Class|KismetSystemLibrary|BoxTraceSingleforObjects _returnvalue _returnvalue "150.000000,100.000000,50.000000" "0, 0, 0" (Utilities|Array|MakeArray "ObjectTypeQuery9") false 0 "ForDuration" true))
  (if _returnvalue_2
    (Class|BPIPlayer|TakeHit(Message) (.HitActor (Collision|BreakHitResult _outhit)))))

(event Custom|Remove%20Trap
  ;[1 1 1] Remove Trap when timer runs out
  (Variables|Default|SetTrapped false)
  (Variables|Default|SetCrawling true)
  (Utilities|FlowControl|Delay 5.0)
  (CallFunction|SetCrawlingHitBox true))

(event Custom|Chase%20Hit%20Box
  (bind _returnvalue (Transformation|GetActorLocation))
  (bind _outhit (Class|KismetSystemLibrary|CapsuleTraceSingleforObjects _returnvalue _returnvalue 2.5e+02 5e+01 (Utilities|Array|MakeArray "ObjectTypeQuery9") false 0 "None" true))
  (if (.bBlockingHit (Collision|BreakHitResult _outhit))
    (Class|BPIPlayer|TakeHit(Message) (.HitActor (Collision|BreakHitResult _outhit)))))

(event Custom|Cancel%20Roaring%20Chase
  ;[1 1 1] Ends Roaring Chase after 20 seconds
  (Variables|Default|SetRoaringChase false)
  (Utilities|Time|ClearandInvalidateTimerbyHandle (Variables|Timers|GetRoaring%20Chase%20Timer%20Handle)))

(event Custom|Set%20X%20Ray
  (params (Active :type Boolean))
  ;[1 1 1] XRay
  (Rendering|SetRenderCustomDepth (Variables|Character|GetMesh) Active))

(event EventBeginPlay
  (Utilities|FlowControl|Sequence
    (:then_0
      (bind _returnvalue (Actor|GetActorOfClass "/Game/GOAP/BP_Planner.BP_Planner_C"))
      (Variables|Default|SetPlanner%20Reference _returnvalue))))

(event EventEvolve
  (params (Evolution%20Selected%20 :type Enum_Evolutions%20Enum :default "NewEnumerator0"))
  (CallFunction|Evolution Evolution%20Selected%20))

(event EventBeginAction
  (params (Action :type Enum_PossibleInvestigations%20Enum :default "NewEnumerator0"))
  (switch Utilities|FlowControl|Switch|SwitchonEnum_PossibleInvestigations Action))

(event EventSetEnemyMoveSpeed
  (params (Action%20Selected :type Enum_Actions%20Enum :default "NewEnumerator0"))
  (Variables|/Script/Engine.CharacterMovementComponent|SetMaxWalkSpeed (Variables|Character|GetCharacterMovement) (Utilities|Select :Index Action%20Selected :NewEnumerator0 3e+02 :NewEnumerator1 3e+02 :NewEnumerator2 5e+02 :NewEnumerator3 5e+02 :NewEnumerator4 5e+04 :NewEnumerator5 0.0 :NewEnumerator6 6e+02 :NewEnumerator7 0.0)))

(event EventSetSelectedInvestigationActor
  (params (Selected%20Investigation :type BP%20Investigation%20Parent%20Object%20Reference))
  (Variables|Default|SetSelected%20Investigation Selected%20Investigation))

(event EventRoaringChaseTimer
  ;[1 1 1] Ends Roaring Chase after 20 seconds
  (bind _returnvalue (Utilities|Time|SetTimerbyEvent (delegate Custom|Cancel%20Roaring%20Chase) 2e+01))
  (Variables|Timers|SetRoaring%20Chase%20Timer%20Handle _returnvalue))

(event EventSetChaseHitBox
  (params (Active :type Boolean))
  (if (not (Variables|Default|GetCrawling))
    (Utilities|Time|SetTimerbyEvent (delegate Custom|Chase%20Hit%20Box) 0.1 Active)))

(event EventSetCrawlingHitBox
  (params (Active :type Boolean))
  ;[1 1 1] Hit box for when enemy is crawling
  (Utilities|Time|SetTimerbyEvent (delegate Custom|Crawl%20Hit%20Trace) 0.1 Active))

(fn ConstructionScript)

(fn Evolution
  (params (Chosen%20Evolution :type Enum_Evolutions%20Enum :default "NewEnumerator0"))
  (Utilities|Map|Add (Variables|Default|GetEvolutions) Chosen%20Evolution true)
  (Class|FMODBlueprintStatics|PlayEvent2D "/Game/FMOD/Events/Bell.Bell")
  (Development|PrintString "Evolved")
  (Class|BPIGamemode|MessageTextPopUpAnimation(Message) (Game|GetGameMode) "NewEnumerator0"))

(fn BearTrapTrigger
  (Variables|Default|SetTrapped true)
  (CallFunction|CancelRoaringChase)
  (CallFunction|SetChaseHitBox false)
  (CallFunction|BeginTrapDuration)
  (Development|PrintString "enemy trap")
  (Class|FMODBlueprintStatics|PlayEventatLocation "/Game/FMOD/Events/Enemy_in_Pain.Enemy_in_Pain" (Math|Transform|MakeTransform (Transformation|GetActorLocation) "0, 0, 0" "1.000000,1.000000,1.000000"))
  (return true))

(fn EnemyTakeHit
  (params (Damage :type Integer))
  (CallFunction|RemoveTrap)
  (if (<= (- (Variables|Default|GetHealth) Damage) 0)
    (Class|FMODBlueprintStatics|PlayEventatLocation "/Game/FMOD/Events/Enemy_Death.Enemy_Death" (Math|Transform|MakeTransform (Transformation|GetActorLocation) "0, 0, 0" "1.000000,1.000000,1.000000"))
    (Variables|Default|SetDead true)
    (return false true)
    (else
      (Class|FMODBlueprintStatics|PlayEventatLocation "/Game/FMOD/Events/Enemy_Hit.Enemy_Hit" (Math|Transform|MakeTransform (Transformation|GetActorLocation) "0, 0, 0" "1.000000,1.000000,1.000000"))
      (return false false))))

(fn GetEnemyKeys
  (return (Variables|Default|GetCan%20See%20Player)))

(fn GetEnemyType
  (return (Variables|Default|GetAgent%20Name)))

(fn GetInvestigationActorThroughActor
  (return 0))

(fn GetPlanner
  (return (Variables|Default|GetPlanner%20Reference)))

(fn GetSelectedInvestigationActor
  (return (Variables|Default|GetSelected%20Investigation)))

(fn SpawnBearTrap
  (return "0, 0, 0" false))